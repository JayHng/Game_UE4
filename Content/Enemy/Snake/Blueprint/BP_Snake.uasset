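; BP_Snake is a snake enemy that carries a health bar widget and loses health when shot.
; On BeginPlay it registers itself as the Owner of its WB_HealthBar widget.
; Capsule hits from a FirstPersonProjectile subtract a fixed amount from HP, with no death handling in these graphs.
; Tick pins the widget to zero world rotation, leaving a look-at-player rotation node unused.
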(event OnComponentHit(CapsuleComponent)
  (params (HitComponent :type Primitive%20Component%20Object%20Reference) (OtherActor :type Actor%20Object%20Reference) (OtherComp :type Primitive%20Component%20Object%20Reference) (NormalImpulse :type Vector :default "0, 0, 0") (Hit :type Hit%20Result%20Structure%20%28by%20ref%29))
  (Utilities|Casting|CastToFirstPersonProjectile OtherActor)
  (Variables|Default|SetHP (- (Variables|Default|GetHP) 1e+01)))

(event EventBeginPlay
  (bind _aswb_health_bar (Utilities|Casting|CastToWB_HealthBar (UserInterface|GetUserWidgetObject (Variables|Default|GetWidget))))
  (Variables|/Game/UI/EnemyHealthBar/WB_HealthBar.WB_HealthBar_C|SetOwner _aswb_health_bar self))

(event Collision|EventActorBeginOverlap
  (params (OtherActor :type Actor%20Object%20Reference)))

(event EventTick
  (params (DeltaSeconds :type Float%20%28single-precision%29))
  (Transformation|SetWorldRotation (Variables|Default|GetWidget) "0, 0, 0" false false))

(fn ConstructionScript)