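; Boss enemy that turns to face the player (FreemanController) on sight, shoots at them and carries a health bar.
; Pawn sensing drives the aim and spawns impulse-launched FirstPersonProjectiles, gated by a flag and a delay as a cooldown.
; Capsule hits from FreemanController itself reduce HP until the boss is destroyed.
; The health bar widget receives the boss as owner and is held at zero world rotation every tick.
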(event OnComponentHit(CapsuleComponent)
  (params (HitComponent :type Primitive%20Component%20Object%20Reference) (OtherActor :type Actor%20Object%20Reference) (OtherComp :type Primitive%20Component%20Object%20Reference) (NormalImpulse :type Vector :default "0, 0, 0") (Hit :type Hit%20Result%20Structure%20%28by%20ref%29))
  (Utilities|Casting|CastToFreemanController OtherActor)
  (Variables|Default|SetHP (- (Variables|Default|GetHP) 0.2))
  (if (<= (Variables|Default|GetHP) 0.0)
    (Actor|DestroyActor self)))

(event OnSeePawn(PawnSensing)
  (params (Pawn :type Pawn%20Object%20Reference))
  (bind _asfreeman_controller (Utilities|Casting|CastToFreemanController Pawn))
  (Utilities|FlowControl|Sequence
    (:then_0
      (Transformation|SetActorRotation (Math|Rotator|FindLookatRotation (Transformation|GetActorLocation) (Transformation|GetActorLocation _asfreeman_controller))))
    (:then_1
      (if (Variables|Default|GetSpawnProjectile)
        (bind _returnvalue (Game|SpawnActorfromClass "/Game/FirstPersonCPP/Blueprints/FirstPersonProjectile.FirstPersonProjectile_C" (Transformation|GetWorldTransform (Variables|Default|GetProjectileSpawnLocation)) "Undefined" 0 0))
        (Physics|AddImpulse (Variables|/Game/FirstPersonCPP/Blueprints/FirstPersonProjectile.FirstPersonProjectile_C|GetStaticMesh1 _returnvalue) (* (Math|Vector|GetForwardVector (Variables|Character|GetMesh)) (Variables|Default|GetshootAmount)) "None" true)
        (Variables|Default|SetSpawnProjectile false)
        (Utilities|FlowControl|Delay 1.0)
        (Variables|Default|SetSpawnProjectile true)))))

(event EventBeginPlay
  (bind _aswb_health_bar_1 (Utilities|Casting|CastToWB_HealthBar1 (UserInterface|GetUserWidgetObject (Variables|Default|GetWidget))))
  (Variables|/Game/UI/EnemyHealthBar/WB_HealthBar1.WB_HealthBar1_C|SetOwner _aswb_health_bar_1 self))

(event EventTick
  (params (DeltaSeconds :type Float%20%28single-precision%29))
  (Transformation|SetWorldRotation (Variables|Default|GetWidget) "0, 0, 0" false false))

(fn ConstructionScript)