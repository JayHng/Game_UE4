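; Second boss enemy that turns to face the player and fires projectiles on sight.
; PawnSensing snaps rotation toward any FreemanController pawn, then launches a FirstPersonProjectile by impulse along the mesh's forward vector, gated by a flag and one-second Delay.
; BeginPlay caches three patrol points and picks a random index, but the timeline logic that would lerp between them never runs, so patrol movement is inactive.
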(event OnSeePawn(PawnSensing)
  (params (Pawn :type Pawn%20Object%20Reference))
  ;[1 1 1] Rotate and Shoot
  (bind _asfreeman_controller (Utilities|Casting|CastToFreemanController Pawn))
  (Utilities|FlowControl|Sequence
    (:then_0
      (Transformation|SetActorRotation (Math|Rotator|FindLookatRotation (Transformation|GetActorLocation) (Transformation|GetActorLocation _asfreeman_controller))))
    (:then_1
      (if (Variables|Default|GetSpawnProjectile)
        (bind _returnvalue (Game|SpawnActorfromClass "/Game/FirstPersonCPP/Blueprints/FirstPersonProjectile.FirstPersonProjectile_C" (Transformation|GetWorldTransform (Variables|Default|GetProjectileSpawnLocation)) "Undefined" 0 0))
        (Physics|AddImpulse (Variables|/Game/FirstPersonCPP/Blueprints/FirstPersonProjectile.FirstPersonProjectile_C|GetStaticMesh1 _returnvalue) (* (Math|Vector|GetForwardVector (Variables|Character|GetMesh)) (Variables|Default|GetshootAmount)) "None" true)
        (Variables|Default|SetSpawnProjectile false)
        (Utilities|FlowControl|Delay 1.0)
        (Variables|Default|SetSpawnProjectile true)))))

(event Collision|EventActorBeginOverlap
  (params (OtherActor :type Actor%20Object%20Reference)))

(event EventTick
  (params (DeltaSeconds :type Float%20%28single-precision%29)))

(event EventBeginPlay
  ;[1 1 1] Patrol
  (Variables|Default|Setpatrollocations (Utilities|Array|MakeArray (Transformation|GetWorldLocation (Variables|Default|GetMovePos3)) (Transformation|GetWorldLocation (Variables|Default|GetMovePos2)) (Transformation|GetWorldLocation (Variables|Default|GetMovePos1))))
  (CallFunction|GetRandomLocation))

(fn ConstructionScript)

(fn GetRandomLocation
  (Variables|Default|Setcurrentpatrolpoint (Math|Random|RandomInteger (Utilities|Array|Length (Variables|Default|Getpatrollocations)))))