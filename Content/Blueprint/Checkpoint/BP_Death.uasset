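; BP_Death is a death trigger that returns the player to the last saved checkpoint.
; Any overlap on DeathTrigger disables input on the player's FreemanController character, without checking the overlapping actor, then waits briefly.
; If the "check" save slot exists, it moves the character to the saved Save_Game location and re-enables input.
; Otherwise it opens the level named by LevelName.
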(event OnComponentBeginOverlap(DeathTrigger)
  (params (OverlappedComponent :type Primitive%20Component%20Object%20Reference) (OtherActor :type Actor%20Object%20Reference) (OtherComp :type Primitive%20Component%20Object%20Reference) (OtherBodyIndex :type Integer) (bFromSweep :type Boolean) (SweepResult :type Hit%20Result%20Structure%20%28by%20ref%29))
  (bind _asfreeman_controller (Utilities|Casting|CastToFreemanController (Game|GetPlayerCharacter 0)))
  (Input|DisableInput _asfreeman_controller (Game|GetPlayerController 0))
  (Utilities|FlowControl|Delay 2.0)
  (bind _returnvalue (SaveGame|DoesSaveGameExist "check"))
  (if _returnvalue
    (bind _returnvalue_2 (SaveGame|LoadGamefromSlot "check"))
    (bind _assave_game (Utilities|Casting|CastToSave_Game _returnvalue_2))
    (bind _asfreeman_controller_2 (Utilities|Casting|CastToFreemanController (Game|GetPlayerCharacter 0)))
    (Transformation|SetActorLocation _asfreeman_controller_2 (Variables|/Game/Blueprint/Checkpoint/Save_Game.Save_Game_C|GetPlayerLoc_S _assave_game) false false)
    (Input|EnableInput _asfreeman_controller_2 (Game|GetPlayerController 0))
    (else
      (Game|OpenLevel(byName) (Variables|Default|GetLevel%20name)))))

(event EventBeginPlay)

(event Collision|EventActorBeginOverlap
  (params (OtherActor :type Actor%20Object%20Reference)))

(event EventTick
  (params (DeltaSeconds :type Float%20%28single-precision%29)))

(fn ConstructionScript)